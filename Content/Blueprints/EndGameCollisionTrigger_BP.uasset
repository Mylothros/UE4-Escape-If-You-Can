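; End-game trigger actor that also runs the level's in-game music.
; On BeginPlay it spawns the IngameBETA 2D sound and fades it in.
; When the player pawn, matched by display name, overlaps the Box, it shows the EndGame widget, fades out the music and pauses the game.
; The Castle stream level unload sits behind a Delay that follows the pause.
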(event OnComponentBeginOverlap(Box)
  (params (OverlappedComponent :type Primitive%20Component%20Object%20Reference) (OtherActor :type Actor%20Object%20Reference) (OtherComp :type Primitive%20Component%20Object%20Reference) (OtherBodyIndex :type Integer) (bFromSweep :type Boolean) (SweepResult :type Hit%20Result%20Structure%20%28by%20ref%29))
  (if (Utilities|Enum|Equal(Enum) (Utilities|GetDisplayName OtherActor) (Utilities|GetDisplayName (Game|Player|GetPlayerPawn 0)))
    (bind _returnvalue (UserInterface|CreateWidget "/Game/Blueprints/Widgets/Menu/EndGame.EndGame_C"))
    (UserInterface|Viewport|AddtoViewport _returnvalue 0)
    (Audio|Components|Audio|FadeOut (Variables|Default|GetCastle) 1.0 0.0 :!class /Script/Engine.AudioComponent)
    (Game|SetGamePaused true)
    (Utilities|FlowControl|Delay 1.5)
    (Game|UnloadStreamLevel(byName) "Castle" false)))

(event EventBeginPlay
  (bind _returnvalue (Audio|SpawnSound2D "/Game/Sounds/ingameBETA.ingameBETA" 1.0 1.0 0.0 0))
  (bind _output_get (Variables|Default|SetCastle _returnvalue))
  (Audio|Components|Audio|FadeIn _returnvalue 2.0 1.0 0.0 :!class /Script/Engine.AudioComponent))

(event Collision|EventActorBeginOverlap
  (params (OtherActor :type Actor%20Object%20Reference)))

(event EventTick
  (params (DeltaSeconds :type Float%20%28single-precision%29)))

(fn ConstructionScript)